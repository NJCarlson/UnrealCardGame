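; BP_CameraPawn is a camera pawn in the CardSystem folder that pans with the WASD keys.
; Key press and release events add or remove direction offsets in a CameraMovement vector.
; Each Tick, MoveCamera normalizes that vector, scales it by a CameraZoom blend between minimum and maximum speeds, and moves the pawn with zero rotation.
; The step ignores delta time, and nothing here changes CameraZoom.
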(event `self.ReceiveBeginPlay`
  (set `self.CameraPawn` self))

(event `self.ReceiveTick`
  (params (DeltaSeconds :type "Float (single-precision)"))
  (`self.MoveCamera`))

(event `Key|W`
  (params (Key :type "Key Structure"))
  (bind _cameramovement (`self.CameraMovement`))
  (:`Pressed`
    (set `self.CameraMovement` (- _cameramovement (-1.0 0.0 0.0))))
  (:`Released`
    (set `self.CameraMovement` (+ _cameramovement (-1.0 0.0 0.0)))))

(event `Key|A`
  (params (Key :type "Key Structure"))
  (bind _cameramovement (`self.CameraMovement`))
  (:`Pressed`
    (set `self.CameraMovement` (- _cameramovement (0.0 1.0 0.0))))
  (:`Released`
    (set `self.CameraMovement` (+ _cameramovement (0.0 1.0 0.0)))))

(event `Key|D`
  (params (Key :type "Key Structure"))
  (bind _cameramovement (`self.CameraMovement`))
  (:`Pressed`
    (set `self.CameraMovement` (- _cameramovement (0.0 -1.0 0.0))))
  (:`Released`
    (set `self.CameraMovement` (+ _cameramovement (0.0 -1.0 0.0)))))

(event `Key|S`
  (params (Key :type "Key Structure"))
  (bind _cameramovement (`self.CameraMovement`))
  (:`Pressed`
    (set `self.CameraMovement` (- _cameramovement (1.0 0.0 0.0))))
  (:`Released`
    (set `self.CameraMovement` (+ _cameramovement (1.0 0.0 0.0)))))

(fn `MoveCamera`
  (bind _camerapawn (`self.CameraPawn`))
  (`WidgetLayoutLibrary.GetMousePositionOnViewport`)
  (`self.K2_SetActorLocationAndRotation` _camerapawn (+ (* (`KismetMathLibrary.Normal` (`self.CameraMovement`)) (`KismetMathLibrary.Lerp` (`self.MinCamSpeed`) (`self.MaxCamSpeed`) (`self.CameraZoom`))) (`self.K2_GetActorLocation` _camerapawn)) (struct) false false))

(fn `UserConstructionScript`)